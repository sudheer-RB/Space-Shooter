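; Player-controlled ship pawn flown by physics forces on its BODY, with an engine that starts only when Fuel exceeds a minimum.
; While the engine is on, Enhanced Input drives forward and vertical thrust along FollowCamera axes as mass-independent acceleration.
; Rotate input applies camera-right force at a computed location, using TorqueStrength.
; Mouse axes feed controller yaw and pitch directly, leaving MouseHandling as an unused stub.
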(event Input|EnhancedActionEvents|EnhancedInputActionIA_EngineStart
  (params (ActionValue :type Boolean) (ElapsedSeconds :type Float%20%28double-precision%29) (TriggeredSeconds :type Float%20%28double-precision%29) (InputAction :type Input%20Action%20Object%20Reference :default "/Game/Ship/Inputs/IA_EngineStart.IA_EngineStart"))
  (CallFunction|EngineFunction))

(event Input|EnhancedActionEvents|EnhancedInputActionIA_MoveForward
  (params (ActionValue :type Float%20%28double-precision%29) (ElapsedSeconds :type Float%20%28double-precision%29) (TriggeredSeconds :type Float%20%28double-precision%29) (InputAction :type Input%20Action%20Object%20Reference :default "/Game/Ship/Inputs/IA_MoveForward.IA_MoveForward"))
  (CallFunction|ThrusterFunction ActionValue))

(event Input|EnhancedActionEvents|EnhancedInputActionIA_Vertical
  (params (ActionValue :type Float%20%28double-precision%29) (ElapsedSeconds :type Float%20%28double-precision%29) (TriggeredSeconds :type Float%20%28double-precision%29) (InputAction :type Input%20Action%20Object%20Reference :default "/Game/Ship/Inputs/IA_Vertical.IA_Vertical"))
  (CallFunction|ThrusterUPDOWN ActionValue))

(event Input|EnhancedActionEvents|EnhancedInputActionIA_Rotate
  (params (ActionValue :type Float%20%28double-precision%29) (ElapsedSeconds :type Float%20%28double-precision%29) (TriggeredSeconds :type Float%20%28double-precision%29) (InputAction :type Input%20Action%20Object%20Reference :default "/Game/Ship/Inputs/IA_Rotate.IA_Rotate"))
  (CallFunction|ThrusterLeftRight ActionValue))

(event Input|MouseEvents|MouseX
  (params (AxisValue :type Float%20%28single-precision%29))
  (Pawn|Input|AddControllerYawInput AxisValue))

(event Input|MouseEvents|MouseY
  (params (AxisValue :type Float%20%28single-precision%29))
  (Pawn|Input|AddControllerPitchInput AxisValue))

(fn ConstructionScript)

(fn EngineFunction
  (if (> (Variables|Default|GetFuel) (Variables|Default|GetMinFuelPercentToStart))
    (Variables|Default|SetbEngineOn true)
    (Development|PrintString "Engine Started")
    (else
      (Development|PrintString "Not Enough Fuel"))))

(fn ThrusterFunction
  (params (ActionValue :type Float%20%28double-precision%29))
  (if (Variables|Default|GetbEngineOn)
    (Development|PrintString "MOVING")
    (Physics|AddForce (Variables|Default|GetBODY) (* (Variables|Default|GetThrustStrength) ActionValue (Math|Vector|GetForwardVector (Variables|Default|GetFollowCamera))) "None" true)))

(fn ThrusterLeftRight
  (params (ActionValue :type Float%20%28double-precision%29))
  (if (Variables|Default|GetbEngineOn)
    (bind _returnvalue (Math|Vector|RotatorfromAxisandAngle (Transformation|GetWorldLocation (Variables|Default|GetBODY)) 9e+01))
    (bind _returnvalue_2 (Math|Rotator|GetRotationXVector _returnvalue))
    (Class|PrimitiveComponent|AddForceatLocation (Variables|Default|GetBODY) (* (Variables|Default|GetTorqueStrength) ActionValue (Math|Vector|GetRightVector (Variables|Default|GetFollowCamera))) _returnvalue_2 "None")))

(fn ThrusterUPDOWN
  (params (ActionValue :type Float%20%28double-precision%29))
  (if (Variables|Default|GetbEngineOn)
    (Development|PrintString "MOVING")
    (Physics|AddForce (Variables|Default|GetBODY) (* (Variables|Default|GetThrustStrength) ActionValue (Math|Vector|GetUpVector (Variables|Default|GetFollowCamera))) "None" true)))

(fn MouseHandling
  (params (Xvalue :type Float%20%28double-precision%29) (Yvalue :type Float%20%28double-precision%29)))