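; BP_Projectile is a weapon projectile that damages what it hits and then destroys itself.
; The construction script applies the Speed variable to ProjectileMovement's initial and max speed and sets the actor's life span, with BeginPlay reapplying the speeds.
; A SphereCollision hit on any actor other than itself or its owner applies Damage, credited to InstigatorActor's instigator controller, before destroying the projectile.
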(event OnComponentHit(SphereCollision)
  (params (HitComponent :type Primitive%20Component%20Object%20Reference) (OtherActor :type Actor%20Object%20Reference) (OtherComp :type Primitive%20Component%20Object%20Reference) (NormalImpulse :type Vector :default "0, 0, 0") (Hit :type Hit%20Result%20Structure%20%28by%20ref%29))
  (if (and (!= OtherActor self) (!= OtherActor (Components|GetOwner)))
    (Game|Damage|ApplyDamage OtherActor (Variables|Default|GetDamage) (Game|GetInstigatorController (Variables|Default|GetInstigatorActor)) self)
    (Actor|DestroyActor)))

(event EventBeginPlay
  (bind _projectilemovement (Variables|Default|GetProjectileMovement))
  (bind _speed (Variables|Default|GetSpeed))
  (Variables|Default|SetLifeSpan (Variables|Default|GetLifeSpan))
  (Variables|/Script/Engine.ProjectileMovementComponent|SetInitialSpeed _projectilemovement _speed)
  (Variables|/Script/Engine.ProjectileMovementComponent|SetMaxSpeed _projectilemovement _speed))

(fn ConstructionScript
  (bind _projectilemovement (Variables|Default|GetProjectileMovement))
  (bind _speed (Variables|Default|GetSpeed))
  (Variables|/Script/Engine.ProjectileMovementComponent|SetInitialSpeed _projectilemovement _speed)
  (Variables|/Script/Engine.ProjectileMovementComponent|SetMaxSpeed _projectilemovement _speed)
  (Actor|SetLifeSpan (Variables|Default|GetLifeSpan)))